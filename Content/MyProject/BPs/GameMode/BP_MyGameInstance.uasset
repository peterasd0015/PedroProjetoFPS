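; BP_MyGameInstance is the game instance that sets up the game's save object on Init.
; It loads BP_SaveGame from the configured slot if a save exists, otherwise it creates a new save object in memory without writing it to disk.
; The result is kept in BPSaveGameRef, and a debug string reports which path ran.
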(event EventInit
  ;[0.07914 0.4323 0.04545] Criar meu game save objeto se não existir um
  (bind _returnvalue (SaveGame|DoesSaveGameExist (Variables|Default|GetSlotName)))
  (if _returnvalue
    (bind _returnvalue_2 (SaveGame|LoadGamefromSlot (Variables|Default|GetSlotName)))
    (bind _asbp_save_game (Utilities|Casting|CastToBP_SaveGame _returnvalue_2))
    (Variables|Default|SetBPSaveGameRef _asbp_save_game)
    (Development|PrintString "Carreguei meu save")
    (else
      (bind _returnvalue_3 (SaveGame|CreateSaveGameObject "/Game/MyProject/BPs/GameMode/BP_SaveGame.BP_SaveGame_C"))
      (Variables|Default|SetBPSaveGameRef _returnvalue_3)
      (Development|PrintString "Criei meu save"))))