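; Pickup weapon actor that notifies an overlapping Player-tagged actor, then disables its physics and collision once collected.
; Fire plays muzzle spark and sound, or an empty-magazine sound, and spawns BPAmmo from the Muzzle socket aimed at the passed hit point.
; Reload waits a set delay, then refills the magazine from capped reserve ammo, which AddAmmo replenishes.
; It sets a Reloading flag, but Fire does not check it.
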(event OnComponentBeginOverlap(weaponTrigger)
  (params (OverlappedComponent :type Primitive%20Component%20Object%20Reference) (OtherActor :type Actor%20Object%20Reference) (OtherComp :type Primitive%20Component%20Object%20Reference) (OtherBodyIndex :type Integer) (bFromSweep :type Boolean) (SweepResult :type Hit%20Result%20Structure%20%28by%20ref%29))
  (if (Actor|ActorHasTag OtherActor "Player")
    (Class|BPIWeapon|WeaponCollected(Message) OtherActor self)))

(event Custom|WeaponCollectedByPlayer
  (bind _myweapon (Variables|Default|GetMyWeapon))
  (Physics|SetSimulatePhysics _myweapon false)
  (Collision|SetCollisionEnabled _myweapon "NoCollision")
  (Collision|SetCollisionEnabled (Variables|Default|GetweaponTrigger) "NoCollision"))

(event Custom|Fire
  (params (hitPoint :type Vector))
  (bind _myweapon (Variables|Default|GetMyWeapon))
  (bind _returnvalue (Transformation|GetSocketTransform _myweapon "Muzzle" "RTS_World"))
  ;[1 0 0] Fire Event
  (CallFunction|WeaponSpark)
  (Development|PrintString (Utilities|String|ToString(Vector) hitPoint))
  (if (== (Variables|Default|GetcurrentAmmo) 0)
    (Development|PrintString "RELOAD")
    (else
      (Math|Integer|DecrementInt (Variables|Default|GetcurrentAmmo)
        (:%20%20
          (Game|SpawnActorfromClass (Variables|Default|GetBP_Ammo) (Math|Transform|MakeTransform (.location _returnvalue) (Math|Rotator|FindLookatRotation (.location _returnvalue) hitPoint) "1.000000,1.000000,1.000000") "Undefined" 0 0))))))

(event Custom|Reload
  ;[1 0 0] Reload
  (if (== (Variables|Default|GetcurrentAmmo) (Variables|Default|GetmaxAmmo))
    (Development|PrintString "MUNICAO NO MAXIMO")
    (elif (== (Variables|Default|GetcurrentExtraAmmo) 0)
      (Development|PrintString "SEM MUNICAO EXTRA")
      (else
        (Variables|Default|Setreloading true)
        (Variables|Default|SetammoNeeded (- (Variables|Default|GetmaxAmmo) (Variables|Default|GetcurrentAmmo)))
        (Utilities|FlowControl|Delay (Variables|Default|GettimeToReload))
        (if (>= (Variables|Default|GetcurrentExtraAmmo) (Variables|Default|GetammoNeeded))
          (Variables|Default|SetcurrentAmmo (Variables|Default|GetmaxAmmo))
          (Variables|Default|SetcurrentExtraAmmo (- (Variables|Default|GetcurrentExtraAmmo) (Variables|Default|GetammoNeeded)))
          (else
            (Variables|Default|SetcurrentAmmo (+ (Variables|Default|GetcurrentAmmo) (Variables|Default|GetcurrentExtraAmmo)))
            (Variables|Default|SetcurrentExtraAmmo 0))))))
  (Variables|Default|Setreloading false))

(event Custom|AddAmmo
  (params (amount :type Integer))
  ;[1 1 1] Ammo collected
  (Variables|Default|SetcurrentExtraAmmo (Math|Integer|Min(Integer) (+ amount (Variables|Default|GetcurrentExtraAmmo)) (Variables|Default|GetmaxExtraAmmo))))

(event EventBeginPlay)

(event Collision|EventActorBeginOverlap
  (params (OtherActor :type Actor%20Object%20Reference)))

(event EventTick
  (params (DeltaSeconds :type Float%20%28single-precision%29)))

(fn ConstructionScript)

(fn WeaponSpark
  (bind _muzzleflash (Variables|Default|GetMuzzleFlash))
  ;[1 1 1] Weapon Spark
  (if (!= (Variables|Default|GetcurrentAmmo) 0)
    (Effects|SpawnEmitteratLocation "/Game/StarterContent/Particles/P_Explosion.P_Explosion" (Transformation|GetWorldLocation _muzzleflash) (Transformation|GetWorldRotation _muzzleflash) "0.100000,0.100000,0.100000")
    (Audio|SpawnSound2D "/Game/StarterContent/Audio/Explosion01.Explosion01" 0.2 1.0 0.0 0)
    (else
      (Audio|SpawnSound2D "/Game/MyProject/SFX/Sons_jogo/Sem_munição_1.Sem_munição_1" 1.2e+03 1.0 0.0 0))))